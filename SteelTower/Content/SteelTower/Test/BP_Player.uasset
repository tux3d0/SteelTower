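; Test player Blueprint for SteelTower that slides BluePawn sideways along its local Y axis from axis input.
; Each Tick scales the input by PlayerSpeed, clamps it between MinMove and MaxMove and applies it as a local offset, without delta-time scaling.
; ChangeMoveDirection overwrites both clamp bounds, so a caller can limit the allowed movement direction.
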(event EventBeginPlay)

(event Collision|EventActorBeginOverlap
  (params (OtherActor :type Actor%20Object%20Reference)))

(event EventTick
  (params (DeltaSeconds :type Float%20%28single-precision%29))
  (Transformation|AddLocalOffset (Variables|Default|GetBluePawn) (Math|Vector|MakeVector 0.0 (Math|Float|Clamp(Float) (* (Class|Actor|GetInputAxisKeyValue) (Variables|Default|GetPlayer_Speed)) (Variables|Default|GetMin_Move) (Variables|Default|GetMax_Move)) 0.0) false false))

(fn ConstructionScript)

(fn ChangeMoveDirection
  (params (Min_Move :type Float%20%28single-precision%29) (Max_Move :type Float%20%28single-precision%29))
  (Variables|Default|SetMin_Move Min_Move)
  (Variables|Default|SetMax_Move Max_Move))