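; Test enemy AI that slides its Player component along X to follow the BP_Test_Ball, apparently as an opposing paddle.
; Every Tick it finds the ball actor, stores its Sphere's relative location and calls ChangeDirection.
; ChangeDirection uses MoveComponentTo toward that X, clamped to a fixed symmetric range, over MoveSpeedOverTime.
; ChangeMoveDirection stores min and max move limits, but the clamp uses hard-coded bounds instead.
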(event Custom|ChangeDirection
  (Components|MoveComponentTo (Variables|Default|GetPlayer) (Math|Vector|MakeVector (Math|Float|Clamp(Float) (.x (Variables|Default|GetEnemyMoveDirection)) -3.5e+02 3.5e+02) 0.0 0.0) "0, 0, 0" false false (Variables|Default|GetMoveSpeedOverTime) false))

(event EventTick
  (params (DeltaSeconds :type Float%20%28single-precision%29))
  (bind _returnvalue (Actor|GetActorOfClass "/Game/SteelTower/Test/BP_Test_Ball.BP_Test_Ball_C"))
  (Utilities|IsValid _returnvalue
    (:Is%20Valid
      (Variables|Default|SetEnemyMoveDirection (Variables|/Script/Engine.SceneComponent|GetRelativeLocation (Variables|/Game/SteelTower/Test/BP_Test_Ball.BP_Test_Ball_C|GetSphere _returnvalue)))
      (CallFunction|ChangeDirection))))

(fn ConstructionScript)

(fn ChangeMoveDirection
  (params (Min_Move :type Float%20%28single-precision%29) (Max_Move :type Float%20%28single-precision%29))
  (Variables|Default|SetMin_Move Min_Move)
  (Variables|Default|SetMax_Move Max_Move))