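; BP_EnemyAI is a test enemy controller that pushes its BluePawn physics component in response to BP_Ball actors.
; Each Tick loops over all balls, snapping to a fixed X and zeroing velocity when Y or X passes a threshold.
; Otherwise it applies an impulse using the X offset to the ball for both X and Y.
; ChangeMoveDirection only stores MinMove and MaxMove, which Tick never reads.
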(event EventTick
  (params (DeltaSeconds :type Float%20%28single-precision%29))
  (bind _returnvalue (Transformation|GetActorLocation))
  (bind _returnvalue_2 (Transformation|GetActorLocation))
  (bind (_x _y _z) (Math|Vector|BreakVector _returnvalue))
  (bind (_x_2 _y_2 _z_2) (Math|Vector|BreakVector _returnvalue_2))
  (bind _outactors (Actor|GetAllActorsOfClass "/Game/SteelTower/Test/BP_Ball.BP_Ball_C"))
  (for _array_element _outactors
    (bind _asbp_ball (Utilities|Casting|CastToBP_Ball _array_element))
    (if (> (.Y (Math|Vector|BreakVector (Transformation|GetActorLocation))) 1e+03)
      (Transformation|SetActorLocation (Math|Vector|MakeVector 1499.0 _y_2 _z_2) false false)
      (Physics|SetPhysicsLinearVelocity (Variables|Default|GetBluePawn) "0, 0, 0" false "None")
      (elif (> (.X (Math|Vector|BreakVector (Transformation|GetActorLocation))) -1e+03)
        (Transformation|SetActorLocation (Math|Vector|MakeVector -1499.0 _y _z) false false)
        (Physics|SetPhysicsLinearVelocity (Variables|Default|GetBluePawn) "0, 0, 0" false "None")
        (else
          (Physics|AddImpulse (Variables|Default|GetBluePawn) (Math|Vector|MakeVector (- (.X (Math|Vector|BreakVector (Transformation|GetActorLocation _asbp_ball))) (.X (Math|Vector|BreakVector (Transformation|GetActorLocation)))) (- (.X (Math|Vector|BreakVector (Transformation|GetActorLocation _asbp_ball))) (.X (Math|Vector|BreakVector (Transformation|GetActorLocation)))) 0.0) "None" false))))))

(fn ConstructionScript)

(fn ChangeMoveDirection
  (params (Min_Move :type Float%20%28single-precision%29) (Max_Move :type Float%20%28single-precision%29))
  (Variables|Default|SetMin_Move Min_Move)
  (Variables|Default|SetMax_Move Max_Move))