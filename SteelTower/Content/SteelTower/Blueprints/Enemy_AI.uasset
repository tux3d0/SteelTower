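; Enemy AI actor that slides its RedPawn component along the X axis to follow the soccer ball.
; BeginPlay sets a custom tick interval, which paces how often the AI updates.
; Each tick looks up the NewBlueprint actor, caches its SoccerBall relative location, and calls Move.
; Move uses a timed MoveComponentTo toward the ball's X coordinate over the OverTime duration.
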(event Custom|Move
  (Components|MoveComponentTo (Variables|Default|GetRedPawn) (Math|Vector|MakeVector (.x (Variables|Default|GetBall_Loc)) 0.0 0.0) "0, 0, 0" false false (Variables|Default|GetOver%20Time) false))

(event EventBeginPlay
  (Actor|Tick|SetActorTickInterval (Variables|Default|GetTick%20Interval)))

(event Collision|EventActorBeginOverlap
  (params (OtherActor :type Actor%20Object%20Reference)))

(event EventTick
  (params (DeltaSeconds :type Float%20%28single-precision%29))
  (bind _returnvalue (Actor|GetActorOfClass "/Game/SteelTower/Blueprints/NewBlueprint.NewBlueprint_C"))
  (Variables|Default|SetBall_Loc (Variables|/Script/Engine.SceneComponent|GetRelativeLocation (Variables|/Game/SteelTower/Blueprints/NewBlueprint.NewBlueprint_C|GetSoccer_Ball _returnvalue)))
  (CallFunction|Move))

(fn ConstructionScript)