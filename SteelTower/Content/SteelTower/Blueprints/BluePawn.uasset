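; BluePawn is a player pawn that slides left and right along a spline and can grab and release physics objects.
; Axis input offsets it sideways, and Tick snaps it back to the nearest spline point.
; The grab action toggles a short forward line trace that attaches simulating components to a PhysicsHandle, whose target follows a scene component each tick.
; Hits on its Box component spawn a Niagara effect.
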(event OnComponentHit(Box)
  (params (HitComponent :type Primitive%20Component%20Object%20Reference) (OtherActor :type Actor%20Object%20Reference) (OtherComp :type Primitive%20Component%20Object%20Reference) (NormalImpulse :type Vector :default "0, 0, 0") (Hit :type Hit%20Result%20Structure%20%28by%20ref%29))
  (Niagara|SpawnSystematLocation "/Game/SteelTower/Particles/NewNiagaraEmitter_System.NewNiagaraEmitter_System" "0, 0, 0"))

(event EventTick
  (params (DeltaSeconds :type Float%20%28single-precision%29))
  (Utilities|FlowControl|Sequence
    (:then_0
      ;[1 1 1] Movement
      (Transformation|AddLocalOffset (Variables|Default|GetBluePawn) (Math|Vector|MakeVector 0.0 (* (Class|Actor|GetInputAxisKeyValue) 1e+01) 0.0) false false))
    (:then_1
      (Transformation|SetWorldLocation (Variables|Default|GetBluePawn) (Spline|FindLocationClosesttoWorldLocation (Variables|/Game/SteelTower/Blueprints/Spline.Spline_C|GetSpline (Variables|Default|GetSpline)) (Transformation|GetWorldLocation (Variables|Default|GetBluePawn)) "World") false true))
    (:then_2
      (Physics|Components|PhysicsHandle|SetTargetLocation (Variables|Default|GetPhysicsHandle) (Transformation|GetWorldLocation (Variables|Default|GetScene))))))

(event EventBeginPlay
  (Transformation|SetWorldLocation (Variables|Default|GetBluePawn) (Spline|FindLocationClosesttoWorldLocation (Variables|/Game/SteelTower/Blueprints/Spline.Spline_C|GetSpline (Variables|Default|GetSpline)) (Transformation|GetWorldLocation (Variables|Default|GetBluePawn)) "World") false true))

(event Input|ActionEvents|InputActionGrab
  (params (Key :type Key%20Structure :default "None"))
  ;[1 1 1] Grab/Release
  (:Pressed
    (if (Variables|Default|GetHolding)
      (CallFunction|ReleaseBall)
      (else
        (CallFunction|GrabBall)))))

(event Input|AxisEvents|InputAxisLeft/Right
  (params (AxisValue :type Float%20%28single-precision%29))
  ;[1 1 1] Movement
  (Transformation|AddLocalOffset (Variables|Default|GetBluePawn) (Math|Vector|MakeVector 0.0 (* AxisValue 1e+01) 0.0) false false))

(fn ConstructionScript)

(fn GrabBall
  (bind _bluepawn (Variables|Default|GetBluePawn))
  (bind _returnvalue (Transformation|GetWorldLocation _bluepawn))
  (bind (_outhit _returnvalue_2) (Collision|LineTraceByChannel _returnvalue (+ (* (Math|Vector|GetForwardVector _bluepawn) 3.5e+02) _returnvalue) "TraceTypeQuery1" false 0 "None"))
  (if _returnvalue_2
    (if (Class|SceneComponent|IsAnySimulatingPhysics (.HitComponent (Collision|BreakHitResult _outhit)))
      (Class|PhysicsHandleComponent|GrabComponentatLocation (Variables|Default|GetPhysicsHandle) (.HitComponent (Collision|BreakHitResult _outhit)) "None" (Transformation|GetWorldLocation (.HitComponent (Collision|BreakHitResult _outhit))))
      (Variables|Default|SetHolding true))))

(fn ReleaseBall
  (Physics|Components|PhysicsHandle|ReleaseComponent (Variables|Default|GetPhysicsHandle))
  (Variables|Default|SetHolding false))