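; BP_New_Player is the player Blueprint, sliding its Bluepawn component along the local Y axis from axis input.
; Each tick scales the input by PlayerSpeed, clamps it between MinMove and MaxMove and applies it as a local offset, without delta-time scaling.
; ChangeMoveDirection replaces those clamp limits, restricting the allowed movement per tick.
; Bluepawn hits play an attached impact sound; an AddImpulse node is left unconnected.
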(event OnComponentHit(Bluepawn)
  (params (HitComponent :type Primitive%20Component%20Object%20Reference) (OtherActor :type Actor%20Object%20Reference) (OtherComp :type Primitive%20Component%20Object%20Reference) (NormalImpulse :type Vector :default "0, 0, 0") (Hit :type Hit%20Result%20Structure%20%28by%20ref%29))
  (Audio|SpawnSoundAttached "/Game/SteelTower/Sounds/Impact.Impact" HitComponent "None" "0, 0, 0" "0, 0, 0" "KeepRelativeOffset" true 1.0 1.0 0.0 0 0))

(event EventTick
  (params (DeltaSeconds :type Float%20%28single-precision%29))
  (Transformation|AddLocalOffset (Variables|Default|GetBluepawn) (Math|Vector|MakeVector 0.0 (Math|Float|Clamp(Float) (* (Class|Actor|GetInputAxisKeyValue) (Variables|Default|GetPlayerSpeed)) (Variables|Default|GetMin%20Move) (Variables|Default|GetMax%20Move)) 0.0) false false))

(event Input|ActionEvents|InputActionForcePush
  (params (Key :type Key%20Structure :default "None")))

(fn ConstructionScript)

(fn ChangeMoveDirection
  (params (Min_Move :type Float%20%28single-precision%29) (Max_Move :type Float%20%28single-precision%29))
  (Variables|Default|SetMin%20Move Min_Move)
  (Variables|Default|SetMax%20Move Max_Move))