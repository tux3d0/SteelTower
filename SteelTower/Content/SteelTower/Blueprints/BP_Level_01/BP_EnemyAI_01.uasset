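; Enemy AI for Level 01 that slides its RedPawn component along Y to track the soccer ball.
; Each Tick finds the Soccer_Ball actor and, if valid, stores its SoccerBall component's relative location.
; ChangeDirection then uses MoveComponentTo to ease toward that Y, clamped to fixed limits, over MoveSpeedOverTime.
; ChangeMoveDirection sets MinMove and MaxMove, but the clamp does not read them.
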(event Custom|ChangeDirection
  (Components|MoveComponentTo (Variables|Default|GetRedPawn) (Math|Vector|MakeVector 0.0 (Math|Float|Clamp(Float) (.y (Variables|Default|GetEnemyMoveDirection)) -1.5e+03 1.5e+03) 0.0) "0, 0, 0" false false (Variables|Default|GetMoveSpeedOverTime) false))

(event EventTick
  (params (DeltaSeconds :type Float%20%28single-precision%29))
  (bind _returnvalue (Actor|GetActorOfClass "/Game/SteelTower/Blueprints/Soccer_Ball.Soccer_Ball_C"))
  (Utilities|IsValid _returnvalue
    (:Is%20Valid
      (Variables|Default|SetEnemyMoveDirection (Variables|/Script/Engine.SceneComponent|GetRelativeLocation (Variables|/Game/SteelTower/Blueprints/Soccer_Ball.Soccer_Ball_C|GetSoccer_Ball _returnvalue)))
      (CallFunction|ChangeDirection))))

(fn ConstructionScript)

(fn ChangeMoveDirection
  (params (Min_Move :type Float%20%28single-precision%29) (Max_Move :type Float%20%28single-precision%29))
  (Variables|Default|SetMin_Move Min_Move)
  (Variables|Default|SetMax_Move Max_Move))